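; Asteroid actor that takes damage from actors tagged "Bullet" and breaks into smaller asteroids.
; Each mesh hit removes a hitpoint, spawns an explosion emitter at the impact and destroys the bullet.
; A hit at zero hitpoints spawns half-scale copies of itself in a Split-driven loop, each with half the starting hitpoints, and destroys the original.
; Velocity-reset nodes for the fragments are present but unconnected.
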(event OnComponentHit(Mesh)
  (params (OtherActor :type Actor%20Object%20Reference) (OtherComp :type Primitive%20Component%20Object%20Reference) (NormalImpulse :type Vector :default "0, 0, 0") (Hit :type Hit%20Result%20Structure%20%28by%20ref%29))
  (if (Actor|ActorHasTag OtherActor "Bullet")
    (if (> (Variables|Default|GetHitpoints) 0)
      (Variables|Default|SetHitpoints (- (Variables|Default|GetHitpoints) 1))
      (Effects|SpawnEmitteratLocation "/Game/Particles/P_Explosion.P_Explosion" (.Location (Collision|BreakHitResult Hit)))
      (Actor|DestroyActor OtherActor :!label _label)
      (else
        (Development|PrintString "Explode!")
        (for _index (range 0 (Variables|Default|GetSplit))
          (bind _returnvalue (Transformation|GetRelativeTransform (Variables|Default|GetRoot)))
          (bind _returnvalue_2 (Game|SpawnActorfromClass "Asteroid_C" (Math|Transform|MakeTransform (.Location (Math|Transform|BreakTransform _returnvalue)) (.Rotation (Math|Transform|BreakTransform _returnvalue)) (* (.Scale (Math|Transform|BreakTransform _returnvalue)) 0.5)) true))
          (Components|StaticMesh|SetStaticMesh (Variables|Asteroid_C|GetMesh _returnvalue_2) (Variables|Default|GetAsteroidMesh))
          (Variables|Asteroid_C|SetHitpoints _returnvalue_2 (/ (Variables|Default|GetdefaultHitpoints) 2))
          (Actor|DestroyActor)
          (goto _label))))))

(fn ConstructionScript
  (Components|StaticMesh|SetStaticMesh (Variables|Default|GetMesh) (Variables|Default|GetAsteroidMesh))
  (Variables|Default|SetdefaultHitpoints (Variables|Default|GetHitpoints)))